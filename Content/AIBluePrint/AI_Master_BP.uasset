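; AI_Master_BP is an AI character with a health HUD widget, a spawned weapon and combat state flags.
; On BeginPlay it spawns the weapon on a back socket, calling OffAll so the player cannot take it.
; A FlipFlop moves the gun between hand and back, while EnableCombat allows firing after the equip montage.
; Damage flags EnemyFound, and head-bone hits or depleted health trigger ragdoll death.
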(event `self.ReceiveBeginPlay`
  (set `self.CurrentHealth` (`self.MaxHealth`))
  (bind _asai_hud (cast `/Game/AIBluePrint/AI_HUD` (`WidgetComponent.GetUserWidgetObject` (`self.Widget`))))
  (set `/Game/AIBluePrint/AI_HUD.Owner` self _asai_hud)
  (`self.SpawnDefaultWeapon`))

(event `EnableCombat`
  (bind _returnvalue (`self.PlayAnimMontage` "/Game/AnimStarterPack/Equip_Rifle_Standing_Montage.Equip_Rifle_Standing_Montage"))
  (`KismetSystemLibrary.Delay` _returnvalue)
  (set `self.CanFire` true))

(event `/Game/AIBluePrint/TakeDamage.ITakeDamage`
  (params (BoneName :type Name) (Damage :type "Float (single-precision)"))
  (if (== (`KismetStringLibrary.Conv_StringToName` (`.RightS` (`KismetStringLibrary.Split` (`KismetStringLibrary.Conv_NameToString` BoneName) "."))) "Head")
    (`KismetSystemLibrary.PrintString` "Head Shot" true true (struct :`R` 0.994792 :`G` 0.989583 :`B` 1.0 :`A` 1.0))
    (set `self.CurrentHealth` 0.0)
    (set `self.IsDead` true :!label _label)
    (`SkeletalMeshComponent.SetAllBodiesSimulatePhysics` (`self.Mesh`) true)
    (`PrimitiveComponent.SetCollisionEnabled` (`self.CapsuleComponent`) "NoCollision")
    (`SceneComponent.SetVisibility` (`self.Widget`) false false)
    (else
      (set `self.EnemyFound` true)
      (bind _output_get (set `self.CurrentHealth` (- (`self.CurrentHealth`) Damage)))
      (if (<= _output_get 0.0)
        (goto _label)))))

(event `Equip/UnEquip`
  (`/Engine/EditorBlueprintResources/StandardMacros.FlipFlop`
    (:`A`
      (`self.K2_AttachToComponent` (`self.WeaponBP`) (`self.Mesh`) "GunHold" "KeepRelative" "KeepRelative" "KeepRelative" true)
      (set `self.EquipWeapon` true))
    (:`B`
      (`self.K2_AttachToComponent` (`self.WeaponBP`) (`self.Mesh`) "Back1" "KeepRelative" "KeepRelative" "KeepRelative" true)
      (set `self.EquipWeapon` false)
      (set `self.EnemyFound` false))))

(event `SpawnDefaultWeapon`
  (bind _returnvalue (`|SpawnActorFromClass` (`self.WeaponClass`) (`SceneComponent.K2_GetComponentToWorld` (`self.Sphere`)) "AlwaysSpawn" "OverrideRootScale" null null))
  (bind _output_get (set `self.WeaponBP` _returnvalue))
  (`self.K2_AttachToComponent` _output_get (`self.Mesh`) "Back1" "KeepWorld" "KeepWorld" "KeepWorld" true)
  ;[1 1 1] 不然主角可以抢NPC的枪
  (`/Game/ThirdPersonBP/Pickups/WeaponPickup/MasterPickupsBP.OffAll` _output_get))

(fn `UserConstructionScript`)